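; Trigger box actor that opens the async save game demo widget (W_SaveGameAsync) when the third-person character overlaps it.
; The first overlap creates the widget and adds it to the viewport; later overlaps show it again and reset its switcher to the first page.
; It then disables the player's movement, switches input to UI only and shows the mouse cursor.
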(event `self.Box.OnComponentBeginOverlap`
  (params (OverlappedComponent :type "PrimitiveComponent Object Reference") (OtherActor :type "Actor Object Reference") (OtherComp :type "PrimitiveComponent Object Reference") (OtherBodyIndex :type Integer) (bFromSweep :type Boolean) (SweepResult :type "HitResult Structure (by ref)"))
  (bind _returnvalue (`GameplayStatics.GetPlayerController` 0))
  (bind _returnvalue_2 (`GameplayStatics.GetPlayerCharacter` 0))
  (cast `TP_ThirdPersonCharacter` OtherActor)
  (`self.Widget`
    (:`then`
      (`Widget.SetVisibility` (`self.Widget`) "Visible")
      (`WidgetSwitcher.SetActiveWidgetIndex` (`/Game/Gym/Widgets/W_SaveGameAsync.WidgetSwitcher_SaveGameAsync` (`self.Widget`)) 0))
    (:`else`
      (bind _returnvalue_3 (`|CreateWidget` "/Game/Gym/Widgets/W_SaveGameAsync.W_SaveGameAsync_C"))
      (bind _output_get (set `self.Widget` _returnvalue_3))
      (`UserWidget.AddToViewport` _output_get 0)))
  (cast `TP_ThirdPersonCharacter` _returnvalue_2)
  (`CharacterMovementComponent.DisableMovement` (`Character.CharacterMovement` _returnvalue_2))
  (`WidgetBlueprintLibrary.SetInputMode_UIOnlyEx` _returnvalue null)
  (set `PlayerController.bShowMouseCursor` true _returnvalue))

(fn `UserConstructionScript`)