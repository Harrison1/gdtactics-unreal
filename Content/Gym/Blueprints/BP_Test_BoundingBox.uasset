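; BP_Test_BoundingBox is a gym test actor that shows a list widget when something overlaps its box.
; On begin overlap, it appends every overlapping BP_Test_Manny to an Actors array, which is never cleared here, then passes the array to a new W_List widget added to the viewport.
; On end overlap, it removes the most recently stored widget from its parent.
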(event `self.Box.OnComponentBeginOverlap`
  (params (OverlappedComponent :type "PrimitiveComponent Object Reference") (OtherActor :type "Actor Object Reference") (OtherComp :type "PrimitiveComponent Object Reference") (OtherBodyIndex :type Integer) (bFromSweep :type Boolean) (SweepResult :type "HitResult Structure (by ref)"))
  (for _array_element (`PrimitiveComponent.GetOverlappingActors` (`self.Box`) "/Game/Gym/Blueprints/BP_Test_Manny.BP_Test_Manny_C")
    (bind _asbp_test_manny (cast `/Game/Gym/Blueprints/BP_Test_Manny` _array_element))
    (`KismetArrayLibrary.Array_Add` (`self.Actors`) _asbp_test_manny))
  (bind _returnvalue (`|CreateWidget` "/Game/Gym/Widgets/W_List.W_List_C" null (`self.Actors`)))
  (bind _output_get (set `self.Widget` _returnvalue))
  (`UserWidget.AddToViewport` _output_get 0))

(event `self.Box.OnComponentEndOverlap`
  (params (OverlappedComponent :type "PrimitiveComponent Object Reference") (OtherActor :type "Actor Object Reference") (OtherComp :type "PrimitiveComponent Object Reference") (OtherBodyIndex :type Integer))
  (`Widget.RemoveFromParent` (`self.Widget`)))

(fn `UserConstructionScript`)