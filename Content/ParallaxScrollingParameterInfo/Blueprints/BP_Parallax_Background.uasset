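; Parallax background actor that scrolls the layers of a plane's material over time.
; The construction script creates a dynamic material instance from the plane's first material.
; Each tick accumulates an offset from velocity and delta time, applying a remainder-by-ten wrap once it exceeds one.
; CreateLayerOffsetArray turns that offset into per-layer name and value pairs, written to the material as scalar parameters.
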(event `self.ReceiveTick`
  (params (DeltaSeconds :type "Float (single-precision)"))
  (set `self.Delta Seconds` DeltaSeconds)
  (set `self.Parallax Offset` (+ (`self.Parallax Offset`) (* (`self.Delta Seconds`) (`self.Parallax Velocity`))))
  (if (> (`self.Parallax Offset`) 1.0)
    (set `self.Parallax Offset` (`KismetMathLibrary.FMod` (`self.Parallax Offset`) 10.0)))
  (`self.UpdateParallaxScrolling` (`self.Parallax Offset`)))

(fn `UpdateParallaxScrolling`
  (params (`Parallax Offset` :type "Float (double-precision)"))
  (bind _returnvalue (`ParallaxScrollingBFL.CreateLayerOffsetArray` (`self.PlaneMID`) `Parallax Offset`))
  (for _array_element _returnvalue
    (bind (_layername _offsetvalue) (break `MyParallaxStruct` _array_element))
    (`MaterialInstanceDynamic.SetScalarParameterValue` (`self.PlaneMID`) _layername _offsetvalue)))

(fn `UserConstructionScript`
  (bind _plane (`self.Plane`))
  (bind _returnvalue (`PrimitiveComponent.CreateDynamicMaterialInstance` _plane 0 (`PrimitiveComponent.GetMaterial` _plane 0) "None"))
  (set `self.PlaneMID` _returnvalue))