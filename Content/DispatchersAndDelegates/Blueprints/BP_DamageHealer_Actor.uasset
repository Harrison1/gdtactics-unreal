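; BP_DamageHealer_Actor is a box-triggered actor that damages, or heals when Heal is set, an actor overlapping it.
; BeginPlay negates BaseDamage for healing, so both modes share the same ApplyDamage call.
; Begin overlap stores the actor, applies damage at once and starts a looping one-second timer on DamageActor.
; Only the latest overlapping actor is tracked, and any end overlap clears the timer.
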(event `self.ReceiveBeginPlay`
  (if (`self.Heal`)
    (set `self.Base Damage` (* (`self.Base Damage`) -1.0))))

(event `DamageActor`
  (`GameplayStatics.ApplyDamage` (`self.Other Actor`) (`self.Base Damage`)))

(event `self.Box.OnComponentBeginOverlap`
  (params (OverlappedComponent :type "PrimitiveComponent Object Reference") (OtherActor :type "Actor Object Reference") (OtherComp :type "PrimitiveComponent Object Reference") (OtherBodyIndex :type Integer) (bFromSweep :type Boolean) (SweepResult :type "HitResult Structure (by ref)"))
  (set `self.Other Actor` OtherActor)
  (`self.DamageActor`)
  (bind _returnvalue (`KismetSystemLibrary.K2_SetTimer` null "DamageActor" 1.0 true))
  (set `self.Timer` _returnvalue))

(event `self.Box.OnComponentEndOverlap`
  (params (OverlappedComponent :type "PrimitiveComponent Object Reference") (OtherActor :type "Actor Object Reference") (OtherComp :type "PrimitiveComponent Object Reference") (OtherBodyIndex :type Integer))
  (`KismetSystemLibrary.K2_ClearAndInvalidateTimerHandle` (`self.Timer`)))

(fn `UserConstructionScript`)